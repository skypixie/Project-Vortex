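; Base actor for destructible environment objects that take weapon damage and explode when their health runs out.
; Point damage reduces HealthComp, whose change event spawns a randomly offset damage-number actor and whose death event destroys the actor with explosion sound and particles.
; Point and radial hits apply the weapon's or projectile's effect according to the mesh material's physical surface type.
; Radial damage only applies that effect and leaves health untouched.
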(event OnHealthChange(HealthComp)
  (params (Health :type Float%20%28single-precision%29) (Damage :type Float%20%28single-precision%29))
  (bind _returnvalue (Game|SpawnActorfromClass "/Game/PVX/Blueprint/InteractionEnvironment/DisplayDamageActor.DisplayDamageActor_C" (Math|Transform|MakeTransform (+ (Transformation|GetActorLocation) (+ (Math|Vector|MakeVector (Math|Random|RandomFloatinRange -4e+01 4e+01) (Math|Random|RandomFloatinRange -4e+01 4e+01) 0.0) (Variables|Default|GetLocalPointSpawnHealthNumber)))) "AlwaysSpawn" "MultiplyWithRoot" 0 0))
  (Default|InitActor _returnvalue Damage Health))

(event OnDead(HealthComp)
  (Actor|DestroyActor))

(event Collision|EventActorBeginOverlap
  (params (OtherActor :type Actor%20Object%20Reference)))

(event EventTick
  (params (DeltaSeconds :type Float%20%28single-precision%29)))

(event Game|Damage|EventAnyDamage
  (params (Damage :type Float%20%28single-precision%29) (DamageType :type Damage%20Type%20Object%20Reference) (InstigatedBy :type Controller%20Object%20Reference) (DamageCauser :type Actor%20Object%20Reference)))

(event Game|Damage|EventPointDamage
  (params (Damage :type Float%20%28single-precision%29) (DamageType :type Damage%20Type%20Object%20Reference) (HitLocation :type Vector :default "0, 0, 0") (HitNormal :type Vector :default "0, 0, 0") (HitComponent :type Primitive%20Component%20Object%20Reference) (BoneName :type Name :default "None") (ShotFromDirection :type Vector :default "0, 0, 0") (InstigatedBy :type Controller%20Object%20Reference) (DamageCauser :type Actor%20Object%20Reference) (HitInfo :type Hit%20Result%20Structure%20%28by%20ref%29))
  (bind _staticmesh (Variables|Default|GetStaticMesh))
  (bind _returnvalue (Rendering|Material|GetMaterial _staticmesh 0))
  (bind _returnvalue_2 (Class|MaterialInterface|GetPhysicalMaterial _returnvalue))
  (bind _surfacetype (Variables|/Script/PhysicsCore.PhysicalMaterial|GetSurfaceType _returnvalue_2))
  (Class|HealthComponent|ChangeHealthValue (Variables|Default|GetHealthComp) (* Damage -1.0))
  (bind _asweapon_default (Utilities|Casting|CastToWeaponDefault DamageCauser))
  (Development|PrintString (Utilities|String|EnumtoString _surfacetype))
  (Class|UserTypes|AddEffectSurfaceType self (.Effect (Utilities|Struct|BreakProjectileInfo (Utilities|Struct|BreakWeaponInfo (Variables|/Script/ProjectVortex.WeaponDefault|GetWeaponSetting _asweapon_default)))) _surfacetype))

(event Game|Damage|EventRadialDamage
  (params (DamageReceived :type Float%20%28single-precision%29) (DamageType :type Damage%20Type%20Object%20Reference) (Origin :type Vector :default "0, 0, 0") (HitInfo :type Hit%20Result%20Structure%20%28by%20ref%29) (InstigatedBy :type Controller%20Object%20Reference) (DamageCauser :type Actor%20Object%20Reference))
  (bind _asprojectile_default (Utilities|Casting|CastToProjectileDefault DamageCauser))
  (Class|UserTypes|AddEffectSurfaceType self (.Effect (Utilities|Struct|BreakProjectileInfo (Variables|/Script/ProjectVortex.ProjectileDefault|GetProjectileSetting _asprojectile_default))) (Variables|/Script/PhysicsCore.PhysicalMaterial|GetSurfaceType (Class|MaterialInterface|GetPhysicalMaterial (Rendering|Material|GetMaterial (Variables|Default|GetStaticMesh) 0)))))

(fn ConstructionScript)

(fn DestroyActor
  (bind _returnvalue (Transformation|GetActorLocation))
  (Actor|DestroyActor)
  (Audio|SpawnSoundatLocation "/Game/StarterContent/Audio/Explosion01.Explosion01" _returnvalue "0, 0, 0" 1.0 1.0 0.0 0 0)
  (Effects|SpawnEmitteratLocation "/Game/StarterContent/Particles/P_Explosion.P_Explosion" _returnvalue))