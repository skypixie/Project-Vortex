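; Game state for PVX that tracks score, lives and level phase progression.
; On BeginPlay it finds the current level's row in DT_Levels and copies its phase score thresholds and final phase.
; IncrementScore updates the first player's score widget, advances the phase at each threshold and returns true once no phases remain.
; CanPlayerRespawn spends a life and returns whether respawn is allowed, with the current phase as checkpoint.
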(event EventBeginPlay
  (bind _returnvalue (Game|GetCurrentLevelName true))
  (bind _outrownames (DataTable|GetDataTableRowNames "/Game/Table/DT_Levels.DT_Levels"))
  (bind _array_element (Utilities|Array|ForEachLoopwithBreak _outrownames :!label _label)
    (:LoopBody
      (bind _returnvalue_2 (Utilities|GetDataTableRow "/Game/Table/DT_Levels.DT_Levels" _array_element)
        (:then
          (if (== (.LevelName (Utilities|Struct|BreakFLevels _returnvalue_2)) (Utilities|String|StringToName _returnvalue))
            (Variables|Default|SetPhase%20Win%20Score (.PhaseWinScore (Utilities|Struct|BreakFLevels _returnvalue_2)))
            (Variables|Default|SetFinal%20Phase (.FinalPhase (Utilities|Struct|BreakFLevels _returnvalue_2)))
            (goto _label Break)))))))

(event EventTick
  (params (DeltaSeconds :type Float%20%28single-precision%29)))

(fn ConstructionScript)

(fn CanPlayerRespawn
  (bind _coutlives (Variables|Default|GetCoutLives))
  (Math|Integer|DecrementInt _coutlives
    (:%20%20
      (return (>= _coutlives 0) (Variables|Default|GetCurrentPhase)))))

(fn IncrementScore
  (params (ChangeValue :type Integer))
  (bind _phase_win_score (Variables|Default|GetPhase%20Win%20Score))
  (bind _output_get (Variables|Default|SetScore (+ ChangeValue (Variables|Default|GetScore))))
  (bind _asbp_pvxplayer_controller (Utilities|Casting|CastToBP_PVXPlayerController (Game|GetPlayerController 0)))
  (Default|SetScoreText (Variables|/Game/PVX/Blueprint/Widget/WBP_IngameWidget.WBP_IngameWidget_C|GetWBP_Stats (Variables|/Game/PVX/Blueprint/Game/BP_PVXPlayerController.BP_PVXPlayerController_C|GetIngameWidget _asbp_pvxplayer_controller)) _output_get)
  (if (Utilities|Array|IsValidIndex _phase_win_score (Variables|Default|GetCurrentPhase))
    (if (>= (Variables|Default|GetScore) (Utilities|Array|Get(acopy) _phase_win_score (Variables|Default|GetCurrentPhase)))
      (bind _output_get_2 (Variables|Default|SetCurrentPhase (+ (Variables|Default|GetCurrentPhase) 1)))
      (if (Utilities|Array|IsValidIndex (Variables|Default|GetPhase%20Win%20Score) _output_get_2)
        (return false)
        (else
          (return true))))
    (else
      (Development|PrintString "WRONG: Current Phase Not Valid" true true "(R=1.000000,G=0.000000,B=0.016666,A=1.000000)" 5.0))))