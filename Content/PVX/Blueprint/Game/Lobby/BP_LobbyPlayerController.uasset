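; Lobby player controller that sets up the local player's lobby camera, cursor and WBP_LobbyMenu.
; On the host it selects the first DT_Levels row and builds a level button per row, while clients display CurrentLevelByServer.
; Map and color choices are forwarded to BP_GM_LobbyMode, and other events update the menu's level and truncated player name or store the lobby character.
; UpdateMeReady is an empty stub.
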(event Custom|UpdateMeReady)

(event Custom|UpdatePlayerSelectedMap
  (params (CurrentLeveByServer :type Name))
  (bind _asbp_gm_lobby_mode (Utilities|Casting|CastToBP_GM_LobbyMode (Game|GetGameMode)))
  (Default|UpdateLevelName _asbp_gm_lobby_mode CurrentLeveByServer))

(event Custom|UpdateLobbyWidgetOnClient
  (params (Name :type Name))
  (Default|UpdateLevelName (Variables|Default|GetLobbyMenu) Name))

(event Custom|UpdatePlayerName
  (params (InText :type Text))
  (Rendering|Components|TextRender|SetText (Variables|/Game/PVX/Blueprint/Widget/LobbyMenu/WBP_LobbyMenu.WBP_LobbyMenu_C|GetPlayerName_text (Variables|Default|GetLobbyMenu)) (Utilities|Text|ToText(String) (Utilities|String|GetSubstring (Utilities|String|ToString(Text) InText) 0 11))))

(event Custom|SelectedNewColor
  (params (Color :type Material%20Interface%20Object%20Reference))
  (bind _asbp_gm_lobby_mode (Utilities|Casting|CastToBP_GM_LobbyMode (Game|GetGameMode)))
  (Default|UpdateColorforCharacter _asbp_gm_lobby_mode Color self))

(event Custom|SaveLobbyCharacter
  (params (LobbyCharacter :type BP%20Lobby%20Char%20Object%20Reference))
  (Variables|Default|SetLobbyCharacter LobbyCharacter))

(event EventBeginPlay
  (bind _returnvalue (Game|GetPlayerController 0))
  (bind _returnvalue_2 (Networking|IsServer))
  (if (Pawn|IsLocalPlayerController)
    (bind _returnvalue_3 (Actor|GetActorOfClass "/Script/Engine.CameraActor"))
    (Game|Player|SetViewTargetwithBlend _returnvalue _returnvalue_3 0.0 "VTBlend_Linear" 0.0 false)
    (Variables|/Script/Engine.PlayerController|SetbShowMouseCursor _returnvalue true)
    (bind _returnvalue_4 (UserInterface|CreateWidget "/Game/PVX/Blueprint/Widget/LobbyMenu/WBP_LobbyMenu.WBP_LobbyMenu_C" _returnvalue _returnvalue_2))
    (Variables|Default|SetLobbyMenu _returnvalue_4)
    (UserInterface|Viewport|AddtoViewport _returnvalue_4 0)
    (if _returnvalue_2
      (bind _outrownames (DataTable|GetDataTableRowNames "/Game/Table/DT_Levels.DT_Levels"))
      (bind _returnvalue_5 (Utilities|GetDataTableRow "/Game/Table/DT_Levels.DT_Levels" (Utilities|Array|Get(acopy) _outrownames))
        (:then
          (Default|UpdateLevelName (Variables|Default|GetLobbyMenu) (.LevelName (Utilities|Struct|BreakFLevels _returnvalue_5)))
          (CallFunction|UpdatePlayerSelectedMap (.LevelName (Utilities|Struct|BreakFLevels _returnvalue_5)))
          (for _array_element _outrownames
            (bind _returnvalue_6 (Utilities|GetDataTableRow "/Game/Table/DT_Levels.DT_Levels" _array_element)
              (:then
                (bind _returnvalue_7 (UserInterface|CreateWidget "/Game/PVX/Blueprint/Widget/LobbyMenu/WBP_LobbyLevelButton.WBP_LobbyLevelButton_C" 0 (.LevelName (Utilities|Struct|BreakFLevels _returnvalue_6)) (Variables|Default|GetLobbyMenu)))
                (Class|VerticalBox|AddChildtoVerticalBox (Variables|/Game/PVX/Blueprint/Widget/LobbyMenu/WBP_LobbyMenu.WBP_LobbyMenu_C|GetSelectLevelByHost_Box (Variables|Default|GetLobbyMenu)) _returnvalue_7))
              (:RowNotFound
                (Development|PrintString "Check table levels" true true "(R=1.000000,G=0.044680,B=0.000000,A=1.000000)")))))
        (:RowNotFound
          (Development|PrintString "Check table levels" true true "(R=1.000000,G=0.044680,B=0.000000,A=1.000000)")))
      (else
        (Default|UpdateLevelName _returnvalue_4 (Variables|Default|GetCurrentLevelByServer))))))

(event EventTick
  (params (DeltaSeconds :type Float%20%28single-precision%29)))

(fn ConstructionScript)