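; Lobby game mode that tracks joining players, places their lobby characters and launches the selected level.
; PostLogin registers each lobby controller, gives it the current level and spawns a BP_LobbyChar at a free target point, using a map of points as occupancy flags.
; Level changes are pushed to every controller's lobby widget, and LaunchGame runs a servertravel console command.
; Color handling and logout are unimplemented stubs.
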(event Custom|LaunchGame
  (Development|ExecuteConsoleCommand (Utilities|String|Append "servertravel " (Utilities|String|ToString(Name) (Variables|Default|GetSelectedLevel))) (Game|GetPlayerController 0)))

(event Custom|SaveColorsForPlayers)

(event Custom|UpdateLevelName
  (params (SelectedLevel :type Name))
  (Variables|Default|SetSelectedLevel SelectedLevel)
  (for _array_element (Variables|Default|GetPlayerControllers)
    (bind _asbp_lobby_player_controller (Utilities|Casting|CastToBP_LobbyPlayerController _array_element))
    (Default|UpdateLobbyWidgetonClient _asbp_lobby_player_controller (Variables|Default|GetSelectedLevel))))

(event Custom|UpdateColorForCharacter
  (params (Color :type Material%20Interface%20Object%20Reference) (Controller :type BP%20Lobby%20Player%20Controller%20Object%20Reference)))

(event EventBeginPlay)

(event EventTick
  (params (DeltaSeconds :type Float%20%28single-precision%29)))

(event EventPostLogin
  (params (NewPlayer :type Player%20Controller%20Object%20Reference))
  (bind _targetpoint (Variables|Default|GetTargetPoint))
  (bind _targetpoint_2 (Variables|Default|GetTargetPoint))
  (bind _keys (Utilities|Map|Keys _targetpoint))
  (if (> (Utilities|Array|Length _keys) 0)
    (bind _outactors (Actor|GetAllActorsOfClass "/Script/Engine.TargetPoint"))
    (for _array_element _outactors
      (Utilities|Map|Add _targetpoint _array_element false)))
  (bind _asbp_lobby_player_controller (Utilities|Casting|CastToBP_LobbyPlayerController NewPlayer))
  (Utilities|Array|Add (Variables|Default|GetPlayerControllers) _asbp_lobby_player_controller)
  (Variables|/Game/PVX/Blueprint/Game/Lobby/BP_LobbyPlayerController.BP_LobbyPlayerController_C|SetCurrentLevelByServer _asbp_lobby_player_controller (Variables|Default|GetSelectedLevel))
  (bind _keys_2 (Utilities|Map|Keys _targetpoint_2))
  (bind _array_element_2 (Utilities|Array|ForEachLoopwithBreak _keys_2 :!label _label)
    (:LoopBody
      (if (not (.Value (Utilities|Map|Find _targetpoint_2 _array_element_2)))
        (Utilities|Map|Add _targetpoint_2 0 false)
        (bind _returnvalue (Game|SpawnActorfromClass "/Game/PVX/Blueprint/Game/Lobby/BP_LobbyChar.BP_LobbyChar_C" (Transformation|GetActorTransform _array_element_2) "AdjustIfPossibleButAlwaysSpawn" "MultiplyWithRoot" 0 0))
        (Variables|/Game/PVX/Blueprint/Game/Lobby/BP_LobbyPlayerController.BP_LobbyPlayerController_C|SetOccupiedPoint _asbp_lobby_player_controller _array_element_2)
        (Default|SaveLobbyCharacter _asbp_lobby_player_controller _returnvalue)
        (CallFunction|SetRandomColorforCharacter _asbp_lobby_player_controller)
        (goto _label Break)))))

(event EventOnLogout
  (params (ExitingController :type Controller%20Object%20Reference)))

(fn ConstructionScript)

(fn SetRandomColorforCharacter
  (params (Controller :type BP%20Lobby%20Player%20Controller%20Object%20Reference))
  (Utilities|Casting|CastToBP_LobbyState (Game|GetGameState)))