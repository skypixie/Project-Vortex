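; BP_Character is the top-down player character, handling weapon pickup swapping and dropping, damage feedback, death and camera.
; InventoryComp loads from PlayerState on BeginPlay and saves back on unpossess, while four input actions swap pickups into slots.
; CharHealthComp drives blood and shield-break effects, and death requests a GameMode respawn.
; It also reports periodic AI noise, multicasts character material, and provides timer-stepped camera zoom and shake.
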(event OnHealthChange(CharHealthComp)
  (params (Health :type Float%20%28single-precision%29) (Damage :type Float%20%28single-precision%29))
  (bind _returnvalue (Math|Float|MapRangeClamped Health 5e+01 1e+02 1.0 0.0))
  (bind _mesh (Variables|Character|GetMesh))
  (bind _returnvalue_2 (Rendering|Material|GetMaterial _mesh 0))
  ;[1 1 1] Blood FX
  (Utilities|FlowControl|Sequence
    (:then_0
      (if (< Damage 0.0)
        (if (> (Math|Random|RandomFloat) 0.7)
          (Rendering|Decal|SpawnDecalatLocation (Utilities|Select :Index (Math|Random|RandomIntegerinRange 0 2) :Option%200 "/Game/MS_Blood/Decal/02_Blood_Stain_sg3bdgoc/02_Blood_Stain_sg3bdgoc_8K_inst.02_Blood_Stain_sg3bdgoc_8K_inst" :Option%201 "/Game/MS_Blood/Decal/03_Blood_Stain_shdwbbkc/03_Blood_Stain_shdwbbkc_8K_inst.03_Blood_Stain_shdwbbkc_8K_inst" :Option%202 "/Game/MS_Blood/Decal/04_Blood_Stain_sheuchmc/04_Blood_Stain_sheuchmc_8K_inst.04_Blood_Stain_sheuchmc_8K_inst") "30.000000,60.000000,60.000000" (+ (Transformation|GetActorLocation) (Math|Vector|MakeVector (Math|Random|RandomFloatinRange -32.0 -32.0) (Math|Random|RandomFloatinRange -32.0 32.0) -1e+02)) "-90.000000,0.000000,0.000000" 2e+01))))
    (:then_1
      (bind _asmaterial_instance_dynamic (Utilities|Casting|CastToMaterialInstanceDynamic _returnvalue_2)
        (:then
          (Rendering|Material|SetScalarParameterValue _asmaterial_instance_dynamic "Blood" _returnvalue :!class /Script/Engine.MaterialInstanceDynamic))
        (:CastFailed
          (bind _returnvalue_3 (Rendering|Material|CreateDynamicMaterialInstance _returnvalue_2 "BloodDynamic" "None" :!class /Script/Engine.KismetMaterialLibrary))
          (Rendering|Material|SetScalarParameterValue _returnvalue_3 "BloodDynamic" _returnvalue :!class /Script/Engine.MaterialInstanceDynamic)
          (Rendering|Material|SetMaterial _mesh 0 _returnvalue_3))))))

(event OnShieldBreak(CharHealthComp)
  ;[1 1 1] Shield FX
  (Effects|SpawnEmitterAttached "/Game/InfinityBladeEffects/P_Cube_Mesh_Test.P_Cube_Mesh_Test" (Variables|Character|GetMesh) "root" "0, 0, 0" "0, 0, 0" "0.500000,0.500000,0.500000" "SnapToTargetIncludingScale"))

(event Custom|StartSwitchWeapon
  (params (Catch%20PickUpWeapon :type BP%20Pick%20Up%20Weapon%20Object%20Reference))
  (bind _returnvalue (UserInterface|CreateWidget "/Game/PVX/Blueprint/Widget/Inventory/WBP_SwitchWeapon.WBP_SwitchWeapon_C"))
  (UserInterface|Viewport|AddtoViewport _returnvalue 0)
  (Variables|Default|SetCatchPickUpWeapon Catch%20PickUpWeapon))

(event Custom|EndSwitchWeapon
  (Variables|Default|SetCatchPickUpWeapon 0))

(event Custom|NoiseEvent
  (Class|AISenseHearing|ReportNoiseEvent (Transformation|GetActorLocation) 1.0 self 0.0 "None"))

(event Custom|SetColorCharacter_OnServer
  (params (TrueColor :type Material%20Interface%20Object%20Reference))
  (CallFunction|SetColorCharacterMulticast TrueColor))

(event Custom|SetColorCharacter_Multicast
  (params (TrueColor :type Material%20Interface%20Object%20Reference))
  (Rendering|Material|SetMaterial (Variables|Character|GetMesh) 0 TrueColor)
  (Variables|Default|SetTrueColor TrueColor))

(event Input|EnhancedActionEvents|EnhancedInputActionIA_Action1
  (params (ActionValue :type Boolean) (ElapsedSeconds :type Float%20%28double-precision%29) (TriggeredSeconds :type Float%20%28double-precision%29) (InputAction :type Input%20Action%20Object%20Reference :default "/Game/PVX/Blueprint/Character/Input/Actions/IA_Action1.IA_Action1"))
  (:Started
    (Class|ProjectVortexCharacter|SetCurrentIndextoSwitch)
    (Utilities|IsValid (Variables|Default|GetCatchPickUpWeapon)
      (:Is%20Valid
        (if (> (Variables|Default|GetCurrentIndexToSwitch) (- (Utilities|Array|Length (Variables|/Script/ProjectVortex.InventoryComponent|GetWeaponSlots (Variables|Default|GetInventoryComp))) 1))
          (Development|PrintString "Error Not correct index" true true "(R=1.000000,G=0.008842,B=0.000000,A=1.000000)")
          (elif (== "" (Variables|/Game/PVX/Blueprint/InteractionEnvironment/PickUps/BP_PickUp_Weapon.BP_PickUp_Weapon_C|GetItemName (Variables|Default|GetCatchPickUpWeapon)))
            (Development|PrintString "Error Not correct WeaponName PickUpActor" true true "(R=1.000000,G=0.000000,B=0.042602,A=1.000000)")
            (else
              (bind (_dropiteminfo _returnvalue) (Class|InventoryComponent|SwitchWeapontoInventory (Variables|Default|GetInventoryComp) (.WeaponInfo (Utilities|Struct|BreakDropItem (Variables|/Game/PVX/Blueprint/InteractionEnvironment/PickUps/BP_PickUp_Weapon.BP_PickUp_Weapon_C|GetWeaponInfo (Variables|Default|GetCatchPickUpWeapon)))) (Variables|Default|GetCurrentIndexToSwitch) (Variables|Default|GetCurrentIndexWeapon)))
              (if _returnvalue
                (CallFunction|DropItem _dropiteminfo)
                (Default|PickUpSuccess (Variables|Default|GetCatchPickUpWeapon))
                (Variables|Default|SetCatchPickUpWeapon 0)))))))))

(event Input|EnhancedActionEvents|EnhancedInputActionIA_Action2
  (params (ActionValue :type Boolean) (ElapsedSeconds :type Float%20%28double-precision%29) (TriggeredSeconds :type Float%20%28double-precision%29) (InputAction :type Input%20Action%20Object%20Reference :default "/Game/PVX/Blueprint/Character/Input/Actions/IA_Action2.IA_Action2"))
  (:Started
    (Class|ProjectVortexCharacter|SetCurrentIndextoSwitch 1)
    (Utilities|IsValid (Variables|Default|GetCatchPickUpWeapon)
      (:Is%20Valid
        (if (> (Variables|Default|GetCurrentIndexToSwitch) (- (Utilities|Array|Length (Variables|/Script/ProjectVortex.InventoryComponent|GetWeaponSlots (Variables|Default|GetInventoryComp))) 1))
          (Development|PrintString "Error Not correct index" true true "(R=1.000000,G=0.008842,B=0.000000,A=1.000000)")
          (elif (== "" (Variables|/Game/PVX/Blueprint/InteractionEnvironment/PickUps/BP_PickUp_Weapon.BP_PickUp_Weapon_C|GetItemName (Variables|Default|GetCatchPickUpWeapon)))
            (Development|PrintString "Error Not correct WeaponName PickUpActor" true true "(R=1.000000,G=0.000000,B=0.042602,A=1.000000)")
            (else
              (bind (_dropiteminfo _returnvalue) (Class|InventoryComponent|SwitchWeapontoInventory (Variables|Default|GetInventoryComp) (.WeaponInfo (Utilities|Struct|BreakDropItem (Variables|/Game/PVX/Blueprint/InteractionEnvironment/PickUps/BP_PickUp_Weapon.BP_PickUp_Weapon_C|GetWeaponInfo (Variables|Default|GetCatchPickUpWeapon)))) (Variables|Default|GetCurrentIndexToSwitch) (Variables|Default|GetCurrentIndexWeapon)))
              (if _returnvalue
                (CallFunction|DropItem _dropiteminfo)
                (Default|PickUpSuccess (Variables|Default|GetCatchPickUpWeapon))
                (Variables|Default|SetCatchPickUpWeapon 0)))))))))

(event Input|EnhancedActionEvents|EnhancedInputActionIA_Action3
  (params (ActionValue :type Boolean) (ElapsedSeconds :type Float%20%28double-precision%29) (TriggeredSeconds :type Float%20%28double-precision%29) (InputAction :type Input%20Action%20Object%20Reference :default "/Game/PVX/Blueprint/Character/Input/Actions/IA_Action3.IA_Action3"))
  (:Started
    (Class|ProjectVortexCharacter|SetCurrentIndextoSwitch 2)
    (Utilities|IsValid (Variables|Default|GetCatchPickUpWeapon)
      (:Is%20Valid
        (if (> (Variables|Default|GetCurrentIndexToSwitch) (- (Utilities|Array|Length (Variables|/Script/ProjectVortex.InventoryComponent|GetWeaponSlots (Variables|Default|GetInventoryComp))) 1))
          (Development|PrintString "Error Not correct index" true true "(R=1.000000,G=0.008842,B=0.000000,A=1.000000)")
          (elif (== "" (Variables|/Game/PVX/Blueprint/InteractionEnvironment/PickUps/BP_PickUp_Weapon.BP_PickUp_Weapon_C|GetItemName (Variables|Default|GetCatchPickUpWeapon)))
            (Development|PrintString "Error Not correct WeaponName PickUpActor" true true "(R=1.000000,G=0.000000,B=0.042602,A=1.000000)")
            (else
              (bind (_dropiteminfo _returnvalue) (Class|InventoryComponent|SwitchWeapontoInventory (Variables|Default|GetInventoryComp) (.WeaponInfo (Utilities|Struct|BreakDropItem (Variables|/Game/PVX/Blueprint/InteractionEnvironment/PickUps/BP_PickUp_Weapon.BP_PickUp_Weapon_C|GetWeaponInfo (Variables|Default|GetCatchPickUpWeapon)))) (Variables|Default|GetCurrentIndexToSwitch) (Variables|Default|GetCurrentIndexWeapon)))
              (if _returnvalue
                (CallFunction|DropItem _dropiteminfo)
                (Default|PickUpSuccess (Variables|Default|GetCatchPickUpWeapon))
                (Variables|Default|SetCatchPickUpWeapon 0)))))))))

(event Input|EnhancedActionEvents|EnhancedInputActionIA_Action4
  (params (ActionValue :type Boolean) (ElapsedSeconds :type Float%20%28double-precision%29) (TriggeredSeconds :type Float%20%28double-precision%29) (InputAction :type Input%20Action%20Object%20Reference :default "/Game/PVX/Blueprint/Character/Input/Actions/IA_Action4.IA_Action4"))
  (:Started
    (Class|ProjectVortexCharacter|SetCurrentIndextoSwitch 3)
    (Utilities|IsValid (Variables|Default|GetCatchPickUpWeapon)
      (:Is%20Valid
        (if (> (Variables|Default|GetCurrentIndexToSwitch) (- (Utilities|Array|Length (Variables|/Script/ProjectVortex.InventoryComponent|GetWeaponSlots (Variables|Default|GetInventoryComp))) 1))
          (Development|PrintString "Error Not correct index" true true "(R=1.000000,G=0.008842,B=0.000000,A=1.000000)")
          (elif (== "" (Variables|/Game/PVX/Blueprint/InteractionEnvironment/PickUps/BP_PickUp_Weapon.BP_PickUp_Weapon_C|GetItemName (Variables|Default|GetCatchPickUpWeapon)))
            (Development|PrintString "Error Not correct WeaponName PickUpActor" true true "(R=1.000000,G=0.000000,B=0.042602,A=1.000000)")
            (else
              (bind (_dropiteminfo _returnvalue) (Class|InventoryComponent|SwitchWeapontoInventory (Variables|Default|GetInventoryComp) (.WeaponInfo (Utilities|Struct|BreakDropItem (Variables|/Game/PVX/Blueprint/InteractionEnvironment/PickUps/BP_PickUp_Weapon.BP_PickUp_Weapon_C|GetWeaponInfo (Variables|Default|GetCatchPickUpWeapon)))) (Variables|Default|GetCurrentIndexToSwitch) (Variables|Default|GetCurrentIndexWeapon)))
              (if _returnvalue
                (CallFunction|DropItem _dropiteminfo)
                (Default|PickUpSuccess (Variables|Default|GetCatchPickUpWeapon))
                (Variables|Default|SetCatchPickUpWeapon 0)))))))))

(event EventWeaponReloadStartBP
  (params (Anim :type Anim%20Montage%20Object%20Reference))
  (|CallParentFunction Anim))

(event EventWeaponReloadEndBP
  (params (bIsSuccess :type Boolean))
  (bind _asabp_ue4character (Utilities|Casting|CastToABP_UE4Character (Components|SkeletalMesh|GetAnimInstance (Variables|Character|GetMesh))))
  (Default|ReloadEnd _asabp_ue4character bIsSuccess))

(event EventWeaponFireStartBP
  (params (Anim :type Anim%20Montage%20Object%20Reference))
  (|CallParentFunction Anim))

(event Game|Damage|EventAnyDamage
  (params (Damage :type Float%20%28single-precision%29) (DamageType :type Damage%20Type%20Object%20Reference) (InstigatedBy :type Controller%20Object%20Reference) (DamageCauser :type Actor%20Object%20Reference))
  (Class|HealthComponent|ChangeHealthValue (Variables|Default|GetCharHealthComp) (* Damage -1.0)))

(event EventCharDeadBP
  ;[1 1 1] Death
  (Collision|SetCollisionResponsetoChannel (Variables|Default|GetCapsuleComponent) "ECC_Pawn" "ECR_Ignore")
  (Actor|SetLifeSpan (Variables|Default|GetCurrentWeapon) 1.0)
  (Actor|SetLifeSpan 1.0)
  (bind _asgm_project_vortex (Utilities|Casting|CastToGM_ProjectVortex (Game|GetGameMode)))
  (bind _bissuccess (Default|TrytoRespawn _asgm_project_vortex))
  (if (not _bissuccess)
    (Default|ShowWinWidget _asgm_project_vortex false)))

(event EventDropWeapontoWorld
  (params (DropItemInfo :type Drop%20Item%20Structure))
  (|CallParentFunction DropItemInfo)
  (CallFunction|DropItem DropItemInfo))

(event EventUnpossessed
  (params (OldController :type Controller%20Object%20Reference))
  (bind _inventorycomp (Variables|Default|GetInventoryComp))
  (bind _asbp_player_state (Utilities|Casting|CastToBP_PlayerState (Variables|/Script/Engine.Controller|GetPlayerState OldController)))
  (bind _returnvalue (Class|InventoryComponent|GetWeaponSlots _inventorycomp))
  (bind _returnvalue_2 (Class|InventoryComponent|GetAmmoSlots _inventorycomp))
  (Default|SaveCurrentInventory _asbp_player_state _returnvalue _returnvalue_2)
  (bind _asbp_pvxplayer_controller (Utilities|Casting|CastToBP_PVXPlayerController OldController))
  (Default|UnbindAllEvents (Variables|/Game/PVX/Blueprint/Widget/WBP_IngameWidget.WBP_IngameWidget_C|GetWBP_InventoryStats (Variables|/Game/PVX/Blueprint/Game/BP_PVXPlayerController.BP_PVXPlayerController_C|GetIngameWidget _asbp_pvxplayer_controller)) self))

(event EventBeginPlay
  (bind _returnvalue (Game|GetPlayerController 0))
  (Utilities|FlowControl|Sequence
    (:then_0
      (bind _asbp_player_state (Utilities|Casting|CastToBP_PlayerState (Variables|/Script/Engine.Controller|GetPlayerState _returnvalue)))
      (Class|InventoryComponent|InitInventory (Variables|Default|GetInventoryComp) (Variables|/Game/PVX/Blueprint/Game/BP_PlayerState.BP_PlayerState_C|GetWeaponSlots _asbp_player_state) (Variables|/Game/PVX/Blueprint/Game/BP_PlayerState.BP_PlayerState_C|GetAmmoSlots _asbp_player_state))
      (bind _asbp_pvxplayer_controller (Utilities|Casting|CastToBP_PVXPlayerController _returnvalue))
      (Default|InitInventoryStateWidget (Variables|/Game/PVX/Blueprint/Widget/WBP_IngameWidget.WBP_IngameWidget_C|GetWBP_InventoryStats (Variables|/Game/PVX/Blueprint/Game/BP_PVXPlayerController.BP_PVXPlayerController_C|GetIngameWidget _asbp_pvxplayer_controller)) self)
      (Utilities|Time|SetTimerbyEvent (delegate Custom|NoiseEvent) 1.0 true))
    (:then_1
      (if (Utilities|Enum|Equal(Enum) (Networking|GetLocalRole) "ROLE_SimulatedProxy")
        (Rendering|Material|SetMaterial (Variables|Character|GetMesh) 0 (Variables|Default|GetTrueColor))))))

(fn ConstructionScript
  (bind _cameraboom (Variables|Default|GetCameraBoom))
  (Variables|/Script/Engine.SpringArmComponent|SetTargetArmLength _cameraboom (Variables|Camera|Main|GetHeight))
  (Transformation|SetRelativeRotation _cameraboom (Variables|Camera|Main|GetRotatorCamera) false false)
  (Variables|/Script/Engine.SpringArmComponent|SetbEnableCameraLag _cameraboom (Variables|Camera|Main|GetFlow))
  (Variables|/Script/Engine.SpringArmComponent|SetCameraLagSpeed _cameraboom (Variables|Camera|Main|GetSmoothCoef)))

(fn CameraShakeEvent
  (Camera|PlayWorldCameraShake "/Game/PVX/Blueprint/Game/BP_CameraShake.BP_CameraShake_C" (Transformation|GetWorldLocation (Variables|Default|GetTopDownCameraComponent)) 0.0 3e+01))

(fn CameraSlideSmooth
  (params (Value :type Float%20%28double-precision%29))
  (bind _cameraboom (Variables|Default|GetCameraBoom))
  (bind _heightcamerachangedistance (Variables|Camera|Slide|GetHeightCameraChangeDistance))
  (bind _targetarmlength (Variables|/Script/Engine.SpringArmComponent|GetTargetArmLength _cameraboom))
  (if (and (!= Value 0.0) (Variables|Camera|Slide|GetSlideDone))
    (if (> Value 0.0)
      (if (>= (Variables|Camera|Main|GetMaxHeight) (+ _heightcamerachangedistance _targetarmlength))
        (Variables|Camera|Slide|SetSlideUp true)
        (Variables|Camera|Slide|SetSlideDone false :!label _label)
        (bind _returnvalue (Utilities|Time|SetTimerbyFunctionName 0 "CameraSlideSmoothTick" (Variables|Camera|Slide|GetTimerStep) true))
        (Variables|Camera|Slide|SetSlideTimer _returnvalue))
      (elif (<= (Variables|Camera|Main|GetMinHeight) (- _targetarmlength _heightcamerachangedistance))
        (Variables|Camera|Slide|SetSlideUp false)
        (goto _label)))))

(fn CameraSlideSmoothTick
  (bind _heightcamerachangeslidestepdistance (Variables|Camera|Slide|GetHeightCameraChangeSlideStepDistance))
  (bind _cameraboom (Variables|Default|GetCameraBoom))
  (bind _output_get (Variables|Camera|Slide|SetCurrentSlideDistance (+ (Variables|Camera|Main|GetHeight) _heightcamerachangeslidestepdistance)))
  (Variables|/Script/Engine.SpringArmComponent|SetTargetArmLength _cameraboom (select (Variables|Camera|Slide|GetSlideUp) (+ (Variables|/Script/Engine.SpringArmComponent|GetTargetArmLength _cameraboom) _heightcamerachangeslidestepdistance) (- (Variables|/Script/Engine.SpringArmComponent|GetTargetArmLength _cameraboom) _heightcamerachangeslidestepdistance)))
  (if (>= _output_get (Variables|Camera|Slide|GetHeightCameraChangeDistance))
    (Variables|Camera|Slide|SetCurrentSlideDistance 0.0)
    (Variables|Camera|Slide|SetSlideDone true)
    (Utilities|Time|ClearandInvalidateTimerbyHandle (Variables|Camera|Slide|GetSlideTimer))))

(fn DropItem
  (params (DropItemInfo :type Drop%20Item%20Structure))
  (bind _returnvalue (Game|SpawnActorfromClass "/Game/PVX/Blueprint/InteractionEnvironment/PickUps/BP_PickUp_Weapon.BP_PickUp_Weapon_C" (Math|Transform|MakeTransform (+ (Transformation|GetActorLocation) (* (Transformation|GetActorForwardVector) 2e+02))) "AdjustIfPossibleButAlwaysSpawn" "MultiplyWithRoot" 0 (.NameItem (Utilities|Struct|BreakWeaponSlot (.WeaponInfo (Utilities|Struct|BreakDropItem DropItemInfo)))) 0))
  (Variables|/Game/PVX/Blueprint/InteractionEnvironment/PickUps/BP_PickUp_Weapon.BP_PickUp_Weapon_C|SetWeaponInfo _returnvalue DropItemInfo))