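; BP_DropItemComponent is an actor component that drops an ammo pickup below its owner.
; Its Drop event traces 1000 units straight down from the owner on the Visibility channel, with debug drawing left on.
; It spawns a BP_PickUp_Ammo slightly above the hit location, passing its weapon ammo type and count.
; The component then destroys itself, so it drops only once.
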(event Custom|Drop
  (bind _returnvalue (Components|GetOwner))
  (bind _returnvalue_2 (Transformation|GetActorLocation _returnvalue))
  (bind _outhit (Collision|LineTraceByChannel _returnvalue_2 (+ _returnvalue_2 "0.000000,0.000000,-1000.000000") "TraceTypeQuery1" false 0 "ForDuration"))
  (Game|SpawnActorfromClass "/Game/PVX/Blueprint/InteractionEnvironment/PickUps/BP_PickUp_Ammo.BP_PickUp_Ammo_C" (Math|Transform|MakeTransform (+ (.Location (Collision|BreakHitResult _outhit)) "0.000000,0.000000,50.000000")) "AdjustIfPossibleButAlwaysSpawn" "MultiplyWithRoot" 0 (Variables|Default|GetType) (Variables|Default|GetCout) 0)
  (Components|DestroyComponent))

(event EventBeginPlay)

(event EventTick
  (params (DeltaSeconds :type Float%20%28single-precision%29)))