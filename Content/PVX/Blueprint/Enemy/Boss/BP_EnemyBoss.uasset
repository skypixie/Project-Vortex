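; Boss enemy Blueprint that extends a parent class with health regeneration and reduced damage scaling on its Health component.
; BeginPlay starts a looping five-second timer, apparently meant to drive RegenerateHP, though the bound function is not shown.
; RegenerateHP briefly raises CoefDamage to full so HPRegenPoints apply unscaled, then sets it back to a low value.
; AnyDamage calls the parent handler, then prints current health.
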(event EventBeginPlay
  (|CallParentFunction)
  (Utilities|Time|SetTimerbyEvent (EventDispatchers|CreateEvent :!event RegenerateHP) 5.0 true))

(event Collision|EventActorBeginOverlap
  (params (OtherActor :type Actor%20Object%20Reference)))

(event EventTick
  (params (DeltaSeconds :type Float%20%28single-precision%29))
  (|CallParentFunction DeltaSeconds) ; This node is disabled and will not be called.\nDrag off pins to build functionality.
)

(event EventAnyDamage
  (params (Damage :type Float%20%28single-precision%29) (DamageType :type Damage%20Type%20Object%20Reference) (InstigatedBy :type Controller%20Object%20Reference) (DamageCauser :type Actor%20Object%20Reference))
  (|CallParentFunction Damage DamageType InstigatedBy DamageCauser)
  (bind _returnvalue (Class|HealthComponent|GetCurrentHealth (Variables|Default|GetHealth)))
  (Development|PrintString (Utilities|String|ToString(Float) _returnvalue)))

(fn ConstructionScript
  (|CallParentFunction))

(fn RegenerateHP
  (bind _health (Variables|Default|GetHealth))
  (Variables|/Script/ProjectVortex.HealthComponent|SetCoefDamage _health 1.0)
  (Class|HealthComponent|ChangeHealthValue _health (Variables|Default|GetHPRegenPoints))
  (Variables|/Script/ProjectVortex.HealthComponent|SetCoefDamage _health 0.2))