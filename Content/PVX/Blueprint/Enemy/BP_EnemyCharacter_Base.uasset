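; Base enemy character with health, melee attacks, hit stun and randomized ammo drops.
; Damage feeds the Health component, which spawns damage displays, may trigger a timed stun and, on death, unpossesses the pawn, drops loot and plays a death montage.
; Random light and heavy montages lock movement and attacks, using notifies to fire debug-drawn sphere traces that damage Player-tagged actors.
; A drop component with random weapon type is rolled at BeginPlay.
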(event OnHealthChange(Health)
  (params (Health :type Float%20%28single-precision%29) (Damage :type Float%20%28single-precision%29))
  (if (not (Variables|Default|GetIsDead))
    (if (> (Variables|Default|GetStunChance) (Math|Random|RandomFloat))
      (CallFunction|StunEnabled))
    (bind _returnvalue (Game|SpawnActorfromClass "/Game/PVX/Blueprint/InteractionEnvironment/DisplayDamageActor.DisplayDamageActor_C" (Math|Transform|MakeTransform (+ (Transformation|GetActorLocation) (+ (Math|Vector|MakeVector (Math|Random|RandomFloatinRange -4e+01 4e+01) (Math|Random|RandomFloatinRange -4e+01 4e+01) 0.0) (Variables|Default|GetSpawnOffsetLocalDamage)))) "AlwaysSpawn" "MultiplyWithRoot" 0 0))
    (Default|InitActor _returnvalue Damage Health)))

(event OnDead(Health)
  (if (not (Variables|Default|GetIsDead))
    (CallFunction|DeadEvent)
    (Animation|Montage|PlayMontage (Variables|Character|GetMesh) (Variables|Default|GetDeadAnim)
      (:OnBlendOut
        (Actor|DestroyActor)))))

(event EventBeginPlay
  (CallFunction|InitDropComponent))

(event EventMeleeAttackLight
  (bind _baselightdamage (Variables|Default|GetBaseLightDamage))
  (bind _lightattackanim (Variables|Default|GetLightAttackAnim))
  (CallFunction|SetStateAttack false)
  (CallFunction|SetStateMovement false)
  (bind _notifyname (Animation|Montage|PlayMontage (Variables|Character|GetMesh) (Utilities|Array|Get(acopy) _lightattackanim (Math|Random|RandomInteger (Utilities|Array|Length _lightattackanim))))
    (:OnCompleted
      (CallFunction|SetStateMovement true :!label _label)
      (CallFunction|SetStateAttack true))
    (:OnInterrupted
      (goto _label))
    (:OnNotifyBegin
      (if (== _notifyname "Attack") ; Light
        (Utilities|MeleeTrace 5e+01 1.5e+02 (Math|Random|RandomFloatinRange (- _baselightdamage 5.0) (+ _baselightdamage 25.0)) (Variables|Default|GetLightRadius))))))

(event EventTick
  (params (DeltaSeconds :type Float%20%28single-precision%29)))

(event Game|Damage|EventAnyDamage
  (params (Damage :type Float%20%28single-precision%29) (DamageType :type Damage%20Type%20Object%20Reference) (InstigatedBy :type Controller%20Object%20Reference) (DamageCauser :type Actor%20Object%20Reference))
  (Class|HealthComponent|ChangeHealthValue (Variables|Default|GetHealth) (* Damage -1.0)))

(event EventMeleeAttackHeavy
  (bind _baseheavydamage (Variables|Default|GetBaseHeavyDamage))
  (bind _heavyattackanim (Variables|Default|GetHeavyAttackAnim))
  (CallFunction|SetStateAttack false)
  (CallFunction|SetStateMovement false)
  (bind _notifyname (Animation|Montage|PlayMontage (Variables|Character|GetMesh) (Utilities|Array|Get(acopy) _heavyattackanim (Math|Random|RandomInteger (Utilities|Array|Length _heavyattackanim))))
    (:OnCompleted
      (CallFunction|SetStateMovement true :!label _label)
      (CallFunction|SetStateAttack true))
    (:OnInterrupted
      (goto _label))
    (:OnNotifyBegin
      (if (== _notifyname "Attack") ; Heavy
        (Utilities|MeleeTrace 5e+01 1.3e+02 (Math|Random|RandomFloatinRange (- _baseheavydamage 1e+01) (+ _baseheavydamage 5e+01)) (Variables|Default|GetHeavyRadius))))))

(fn ConstructionScript)

(fn SetStateMovement
  (params (bCanMove :type Boolean))
  (bind _charactermovement (Variables|Character|GetCharacterMovement))
  (bind _output_get (Variables|Default|SetCanMovePawn bCanMove))
  (if _output_get
    (Variables|/Script/Engine.CharacterMovementComponent|SetMaxWalkSpeed _charactermovement 4e+02)
    (else
      (Variables|/Script/Engine.CharacterMovementComponent|SetMaxWalkSpeed _charactermovement 0.0))))

(fn SetStateAttack
  (params (bCanAttack :type Boolean))
  (Variables|Default|SetCanAttackPawn bCanAttack))

(fn DeadEvent
  (bind _returnvalue (Pawn|GetController))
  (bind _dropcomponent (Variables|Default|GetDropComponent))
  (Utilities|IsValid _returnvalue
    (:Is%20Valid
      (Pawn|UnPossess _returnvalue))
    (:Is%20Not%20Valid
      _))
  (CallFunction|SetStateMovement false)
  (CallFunction|SetStateAttack false)
  (Variables|Default|SetIsDead true)
  (Actor|SetLifeSpan 7.0)
  (Utilities|IsValid _dropcomponent
    (:Is%20Valid
      (Default|Drop _dropcomponent))))

(fn InitDropComponent
  (if (> (Math|Random|RandomFloat) (Variables|Default|GetDropChance))
    (bind _returnvalue (AddComponent|AddBPDropItemComponent))
    (bind _output_get (Variables|Default|SetDropComponent _returnvalue))
    (bind _output_get_2 (Variables|/Game/PVX/Blueprint/BP_DropItemComponent.BP_DropItemComponent_C|SetType _output_get (Utilities|Select :Index (Math|Random|RandomIntegerinRange 0 4) :Option%200 "RifleType" :Option%201 "ShotgunType" :Option%202 "SniperType" :Option%203 "PistolType" :Option%204 "RocketLauncherType")))
    (Utilities|FlowControl|Sequence
      (:then_0
        (switch Utilities|FlowControl|Switch|SwitchonEWeaponType _output_get_2
          (:RifleType
            (Variables|/Game/PVX/Blueprint/BP_DropItemComponent.BP_DropItemComponent_C|SetCout _output_get 30))
          (:ShotgunType
            (Variables|/Game/PVX/Blueprint/BP_DropItemComponent.BP_DropItemComponent_C|SetCout _output_get 12))
          (:SniperType
            (Variables|/Game/PVX/Blueprint/BP_DropItemComponent.BP_DropItemComponent_C|SetCout _output_get 6))
          (:PistolType
            (Variables|/Game/PVX/Blueprint/BP_DropItemComponent.BP_DropItemComponent_C|SetCout _output_get 20))
          (:RocketLauncherType
            (Variables|/Game/PVX/Blueprint/BP_DropItemComponent.BP_DropItemComponent_C|SetCout _output_get 2)))))))

(fn StunEnabled
  (CallFunction|SetStateMovement false)
  (Variables|/Script/Engine.CharacterMovementComponent|SetMaxWalkSpeed (Variables|Character|GetCharacterMovement) 0.0)
  (Utilities|Time|SetTimerbyFunctionName 0 "StunDisableTimer" (Variables|Default|GetStunTimer))
  (Animation|PlayAnimMontage "/Game/Enemies/Girl/Anims/Zombie_Reaction_Hit_Montage.Zombie_Reaction_Hit_Montage" 1.0 "None"))

(fn StunDisableTimer
  (CallFunction|SetStateMovement true)
  (Variables|/Script/Engine.CharacterMovementComponent|SetMaxWalkSpeed (Variables|Character|GetCharacterMovement) 4e+02))

(fn CanAttack
  (return (Variables|Default|GetCanAttackPawn)))

(fn CanMove
  (return (Variables|Default|GetCanMovePawn)))