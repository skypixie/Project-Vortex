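; Ammo pickup actor that gives a character ammo for one weapon type, extending a parent pickup class.
; On BeginPlay it picks the static mesh matching its weapon ammo type and enlarges it, or destroys the mesh component if none is valid.
; When the parent reports a character overlap, it asks the Inventory whether that ammo can be taken, then adds the count and completes the pickup.
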(event EventBeginPlay
  (|CallParentFunction)
  (CallFunction|InitActor))

(event Collision|EventActorBeginOverlap
  (params (OtherActor :type Actor%20Object%20Reference))
  (|CallParentFunction OtherActor) ; This node is disabled and will not be called.\nDrag off pins to build functionality.
)

(event EventTick
  (params (DeltaSeconds :type Float%20%28single-precision%29))
  (|CallParentFunction DeltaSeconds) ; This node is disabled and will not be called.\nDrag off pins to build functionality.
)

(event EventOverlapCharacter
  (params (Inventory :type Inventory%20Component%20Object%20Reference))
  (bind _weapontypeammo (Variables|Default|GetWeaponTypeAmmo))
  (|CallParentFunction Inventory)
  (bind _returnvalue (Class|InventoryComponent|CheckCanTakeAmmo Inventory _weapontypeammo))
  (if _returnvalue
    (Class|InventoryComponent|AmmoSlotChangeValue Inventory _weapontypeammo (Variables|Default|GetCout))
    (CallFunction|PickUpSuccess)))

(fn ConstructionScript
  (|CallParentFunction))

(fn InitActor
  (bind _weapontypeammo (Variables|Default|GetWeaponTypeAmmo))
  (bind _staticmesh (Variables|Default|GetStaticMesh))
  (bind _returnvalue (Utilities|Select :Index _weapontypeammo :RifleType "/Game/MilitaryWeapSilver/Pickups/AssaultRifle_Pickup.AssaultRifle_Pickup" :ShotgunType "/Game/MilitaryWeapSilver/Pickups/Shotgun_Pickup.Shotgun_Pickup" :SniperType "/Game/MilitaryWeapSilver/Pickups/SniperRifle_Pickup.SniperRifle_Pickup" :PistolType "/Game/MilitaryWeapSilver/Pickups/Pistol_Pickup.Pistol_Pickup" :RocketLauncherType "/Game/MilitaryWeapSilver/Pickups/RocketLauncher_Pickup.RocketLauncher_Pickup"))
  (Utilities|IsValid _returnvalue
    (:Is%20Valid
      (Components|StaticMesh|SetStaticMesh _staticmesh _returnvalue)
      (Transformation|SetRelativeScale3D (Variables|Default|GetStaticMesh) "2.000000,2.000000,2.000000"))
    (:Is%20Not%20Valid
      (Components|DestroyComponent _staticmesh))))