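; Weapon pickup actor that offers its weapon to the inventory of an overlapping character.
; On BeginPlay it looks up drop info by ItemName in the game instance, otherwise keeping its existing WeaponInfo, then sets up a static or skeletal mesh and optional VFX, destroying unused components.
; If the inventory accepts the weapon the pickup succeeds; otherwise the character starts weapon switching, which ends on leaving the sphere.
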(event OnComponentEndOverlap(Sphere)
  (params (OverlappedComponent :type Primitive%20Component%20Object%20Reference) (OtherActor :type Actor%20Object%20Reference) (OtherComp :type Primitive%20Component%20Object%20Reference) (OtherBodyIndex :type Integer))
  (bind _asbp_character (Utilities|Casting|CastToBP_Character OtherActor))
  (Default|EndSwitchWeapon _asbp_character))

(event EventBeginPlay
  (bind _itemname (Variables|Default|GetItemName))
  (|CallParentFunction)
  (if (!= _itemname "")
    (bind _asbp_game_instance (Utilities|Casting|CastToBP_GameInstance (Game|GetGameInstance)))
    (bind (_outinfo _returnvalue) (Class|PVXGameInstance|GetDropItemInfobyWeaponName _asbp_game_instance _itemname))
    (if _returnvalue
      (Variables|Default|SetWeaponInfo _outinfo)))
  (CallFunction|InitActor (Variables|Default|GetWeaponInfo)))

(event Collision|EventActorBeginOverlap
  (params (OtherActor :type Actor%20Object%20Reference))
  (|CallParentFunction OtherActor) ; This node is disabled and will not be called.\nDrag off pins to build functionality.
)

(event EventTick
  (params (DeltaSeconds :type Float%20%28single-precision%29))
  (|CallParentFunction DeltaSeconds) ; This node is disabled and will not be called.\nDrag off pins to build functionality.
)

(event EventOverlapCharacter
  (params (Inventory :type Inventory%20Component%20Object%20Reference))
  (|CallParentFunction Inventory)
  (bind _returnvalue (Class|InventoryComponent|TryGetWeapontoInventory Inventory (.WeaponInfo (Utilities|Struct|BreakDropItem (Variables|Default|GetWeaponInfo)))))
  (if _returnvalue
    (CallFunction|PickUpSuccess)
    (else
      (bind _asbp_character (Utilities|Casting|CastToBP_Character (Components|GetOwner Inventory)))
      (Default|StartSwitchWeapon _asbp_character self))))

(fn ConstructionScript
  (|CallParentFunction))

(fn InitActor
  (params (InfoActor :type Drop%20Item%20Structure))
  (bind (_weaponstaticmesh _weaponskeletmesh _particleitem _offset) (Utilities|Struct|BreakDropItem InfoActor))
  (bind _staticmesh (Variables|Default|GetStaticMesh))
  (bind _skeletalmesh (Variables|Default|GetSkeletalMesh))
  (bind _location (Math|Transform|BreakTransform _offset))
  (Utilities|FlowControl|Sequence
    (:then_0
      (Utilities|IsValid _weaponstaticmesh
        (:Is%20Valid
          (Components|DestroyComponent (Variables|Default|GetSkeletalMesh))
          (Components|StaticMesh|SetStaticMesh _staticmesh _weaponstaticmesh)
          (Transformation|SetRelativeLocation _staticmesh _location false false))
        (:Is%20Not%20Valid
          (Utilities|IsValid _weaponskeletmesh
            (:Is%20Valid
              (Components|DestroyComponent (Variables|Default|GetStaticMesh))
              (Components|SkeletalMesh|SetSkeletalMeshAsset _skeletalmesh _weaponskeletmesh)
              (Transformation|SetRelativeLocation _skeletalmesh _location false false))))))
    (:then_1
      (Utilities|IsValid _particleitem
        (:Is%20Valid
          (Effects|Components|ParticleSystem|SetTemplate (Variables|Default|GetVFx) _particleitem))
        (:Is%20Not%20Valid
          (Components|DestroyComponent (Variables|Default|GetVFx)))))))