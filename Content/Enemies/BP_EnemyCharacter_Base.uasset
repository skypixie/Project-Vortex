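; Base enemy Character that takes damage, shows it in the world and handles its own death.
; AnyDamage feeds the Health component while alive, and each health change spawns a display actor at a randomly jittered offset with the damage and current health.
; On death it unpossesses its controller, disables the movement and attack flags, and plays a zombie dying montage.
; The montage's completion or blend-out destroys the actor, alongside a short lifespan.
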(event OnHealthChange(Health)
  (params (Health :type Float%20%28single-precision%29) (Damage :type Float%20%28single-precision%29))
  (bind _returnvalue (Game|SpawnActorfromClass "/Game/PVX/Blueprint/InteractionEnvironment/DisplayDamageActor.DisplayDamageActor_C" (Math|Transform|MakeTransform (+ (Transformation|GetActorLocation) (+ (Math|Vector|MakeVector (Math|Random|RandomFloatinRange -4e+01 4e+01) (Math|Random|RandomFloatinRange -4e+01 4e+01) 0.0) (Variables|Default|GetSpawnOffsetLocalDamage)))) "AlwaysSpawn" "MultiplyWithRoot" 0 0))
  (Default|InitActor _returnvalue Damage Health))

(event OnDead(Health)
  (CallFunction|DeadEvent)
  (Animation|Montage|PlayMontage (Variables|Character|GetMesh) "/Game/Enemies/Girl/Anims/Zombie_Dying_Montage.Zombie_Dying_Montage"
    (:OnCompleted
      _)
    (:OnBlendOut
      _))
  (Actor|DestroyActor))

(event EventBeginPlay)

(event Collision|EventActorBeginOverlap
  (params (OtherActor :type Actor%20Object%20Reference)))

(event EventTick
  (params (DeltaSeconds :type Float%20%28single-precision%29)))

(event Game|Damage|EventAnyDamage
  (params (Damage :type Float%20%28single-precision%29) (DamageType :type Damage%20Type%20Object%20Reference) (InstigatedBy :type Controller%20Object%20Reference) (DamageCauser :type Actor%20Object%20Reference))
  (if (not (Variables|Default|GetIsDead))
    (Class|HealthComponent|ChangeHealthValue (Variables|Default|GetHealth) (* Damage -1.0))))

(fn ConstructionScript)

(fn SetStateMovement
  (params (bCanMove :type Boolean))
  (Variables|Default|SetCanMove bCanMove))

(fn SetStateAttack
  (params (bCanAttack :type Boolean))
  (Variables|Default|SetCanAttack bCanAttack))

(fn DeadEvent
  (bind _returnvalue (Pawn|GetController))
  (Utilities|IsValid _returnvalue
    (:Is%20Valid
      (Pawn|UnPossess _returnvalue))
    (:Is%20Not%20Valid
      _))
  (CallFunction|SetStateMovement false)
  (CallFunction|SetStateAttack false)
  (Variables|Default|SetIsDead true)
  (Actor|SetLifeSpan 4.0))